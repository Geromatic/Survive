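; Base character Blueprint that tracks Health and Stamina, both set to their maximums in the Construction Script.
; When player-controlled, it creates a HUD widget on BeginPlay and updates its health bar as damage is taken.
; At zero health, characters other than the first player stop their AI logic, send a state message to the AnimInstance and make their capsule ignore the Visibility channel.
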(event `self.ReceiveBeginPlay`
  (if (`self.IsPlayerControlled`)
    (bind _returnvalue (`|CreateWidget` "/Game/Blueprints/UserWidget.UserWidget_C"))
    (bind _output_get (set `self.UI_Info` _returnvalue))
    (`UserWidget.AddToViewport` _output_get 0)))

(event `self.ReceiveAnyDamage`
  (params (Damage :type "Float (single-precision)") (DamageType :type "DamageType Object Reference") (InstigatedBy :type "Controller Object Reference") (DamageCauser :type "Actor Object Reference"))
  (set `self.Health` (- (`self.Health`) Damage))
  (`self.ModifyUserHealthUI`)
  (if (and (<= (`self.Health`) 0.0) (!= self (`GameplayStatics.GetPlayerCharacter` 0)))
    (bind _returnvalue (`AIBlueprintHelperLibrary.GetAIController` self))
    (`BrainComponent.StopLogic` (`AIController.BrainComponent` _returnvalue) "Dead")
    (message `/Game/Blueprints/Zombie/IAnim.Set State` (`SkeletalMeshComponent.GetAnimInstance` (`self.Mesh`)) 255)
    (`PrimitiveComponent.SetCollisionResponseToChannel` (`self.CapsuleComponent`) "ECC_Visibility" "ECR_Ignore")))

(fn `Health Percent`
  (returns (value :type "Float (double-precision)"))
  (return (/ (`self.Health`) (`self.Max Health`))))

(fn `ModifyUserHealthUI`
  (if (`self.IsPlayerControlled`)
    (`ProgressBar.SetPercent` (`/Game/Blueprints/UserWidget.Health` (`self.UI_Info`)) (`KismetMathLibrary.FMax` (/ (`self.Health`) (`self.Max Health`)))))
  (return))

(fn `Stamina Percent`
  (returns (value :type "Float (double-precision)"))
  (return (/ (`self.Stamina`) (`self.Max Stamina`))))

(fn `UserConstructionScript`
  (set `self.Health` (`self.Max Health`))
  (set `self.Stamina` (`self.Max Stamina`)))