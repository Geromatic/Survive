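; Behavior Tree service for zombie AI that checks how far the blackboard Target is from the zombie's spawn location.
; On each tick it casts the owner to AIController and its pawn to BP_Zombie to read SpawnLocation.
; When a valid Target is beyond a fixed radius from that point, it writes the same actor back to the Target key, leaving the value unchanged.
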(event `self.ReceiveTick`
  (params (OwnerActor :type "Actor Object Reference") (DeltaSeconds :type "Float (single-precision)"))
  (bind _target (`self.Target`))
  (bind _returnvalue (`BTFunctionLibrary.GetBlackboardValueAsActor` _target))
  (`/Engine/EditorBlueprintResources/StandardMacros.IsValid` _returnvalue
    (:`Is Valid`
      (bind _asaicontroller (cast `AIController` OwnerActor))
      (bind _asbp_zombie (cast `/Game/Blueprints/Zombie/BP_Zombie` (`Controller.K2_GetPawn` _asaicontroller)))
      (if (> (`KismetMathLibrary.VSize` (- (`Actor.K2_GetActorLocation` _returnvalue) (`/Game/Blueprints/Zombie/BP_Zombie.Spawn Location` _asbp_zombie))) 1500.0)
        (`BTFunctionLibrary.SetBlackboardValueAsObject` _target _returnvalue)))))