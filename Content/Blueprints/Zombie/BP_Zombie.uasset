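; BP_Zombie is a zombie enemy that reacts to damage from anything other than another zombie and handles its own death.
; Damage passes to the parent, then a surviving zombie plays its hit montage, messages the AnimInstance and stops moving.
; At zero health it once ignores all collision except WorldStatic, disables AI pawn sensing and further damage, then runs Death.
; A dynamic material's "Evil" parameter is zeroed unless Glow is set, and animated by a death timeline.
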(event `Death`
  (bind (_direction _newtrack_0) (`Timeline|Timeline_0`)
    (:`Update`
      (`MaterialInstanceDynamic.SetScalarParameterValue` (`self.mat`) "Evil" _newtrack_0))))

(event `self.ReceiveBeginPlay`
  (set `self.Spawn Location` (`self.K2_GetActorLocation`)))

(event `self.ReceiveAnyDamage`
  (params (Damage :type "Float (single-precision)") (DamageType :type "DamageType Object Reference") (InstigatedBy :type "Controller Object Reference") (DamageCauser :type "Actor Object Reference"))
  (bind _capsulecomponent (`self.CapsuleComponent`))
  (bind _returnvalue (<= (`self.Health`) 0.0))
  (`self.StopAnimMontage` null)
  (cast `/Game/Blueprints/Zombie/BP_Zombie` DamageCauser
    (:`CastFailed`
      (`parent.ReceiveAnyDamage` Damage DamageType InstigatedBy DamageCauser)
      (`|ExecutionSequence`
        (:`then_0`
          (if (not _returnvalue)
            (`self.PlayAnimMontage` "/Game/Blueprints/Zombie/Lambent_Female/zombie_Montage.zombie_Montage" 1.0 "Hit")
            (message `/Game/Blueprints/Zombie/IAnim.Set State` (`SkeletalMeshComponent.GetAnimInstance` (`self.Mesh`)) 2)
            (`MovementComponent.StopMovementImmediately` (`self.CharacterMovement`))))
        (:`then_1`
          (if _returnvalue
            (`|DoOnceMultiInput`
              (:`A Out`
                (`|ExecutionSequence`
                  (:`then_1`
                    (`PrimitiveComponent.SetCollisionResponseToAllChannels` _capsulecomponent "ECR_Ignore")
                    (`PrimitiveComponent.SetCollisionResponseToChannel` _capsulecomponent "ECC_WorldStatic" "ECR_Block"))
                  (:`then_2`
                    (bind _returnvalue_2 (`AIBlueprintHelperLibrary.GetAIController` self))
                    (bind _asbt_zombie_aicontroller_default (cast `/Game/Blueprints/Zombie/BT_ZombieAIController_Default` _returnvalue_2))
                    (`PawnSensingComponent.SetSensingUpdatesEnabled` (`/Game/Blueprints/Zombie/BT_ZombieAIController_Default.PawnSensing` _asbt_zombie_aicontroller_default) false))
                  (:`then_3`
                    (set `self.bCanBeDamaged` false))
                  (:`then_4`
                    (`self.Death`)))))))))))

(fn `UserConstructionScript`
  (bind _mat (`self.mat`))
  (`parent.UserConstructionScript`)
  (bind _returnvalue (`KismetMaterialLibrary.CreateDynamicMaterialInstance` "/Game/Blueprints/Zombie/Lambent_Female/Mat_zombie.Mat_zombie"))
  (set `self.mat` _returnvalue)
  (if (not (`self.Glow`))
    (`MaterialInstanceDynamic.SetScalarParameterValue` _mat "Evil" 0.0))
  (`PrimitiveComponent.SetMaterial` (`self.Mesh`) 0 _mat))