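; BGlobalFunctions holds a shared helper in the Zombie folder that tests whether a target actor is near the player and facing them.
; DIstanceAndDirectionFromPlayer returns true when player pawn 0 is within the given distance and on the target's forward side.
; The facing test compares only the X signs of the forward vector and the direction to the player, so it works along the world X axis alone.
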(fn `DIstanceAndDirectionFromPlayer`
  (params (Target :type "Actor Object Reference") (Distance :type "Float (double-precision)" :default 300.0))
  (returns (ReturnValue :type Boolean))
  (bind _returnvalue (`GameplayStatics.GetPlayerPawn` null))
  (bind _returnvalue_x (`KismetMathLibrary.BreakVector` (`Actor.GetActorForwardVector` Target)))
  (bind _returnvalue_x_2 (`KismetMathLibrary.BreakVector` (`KismetMathLibrary.GetDirectionUnitVector` (`Actor.K2_GetActorLocation` Target) (`Actor.K2_GetActorLocation` _returnvalue))))
  (return (and (<= (`Actor.GetDistanceTo` Target _returnvalue) Distance) (== (`KismetMathLibrary.SignOfFloat` _returnvalue_x) (`KismetMathLibrary.SignOfFloat` _returnvalue_x_2)))))