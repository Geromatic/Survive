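; A switch that fires a one-time trigger event when the player presses it, waking tagged zombie AI and signaling lights.
; Each press plays a pickup sound, but a DoOnce limits the triggering to the first press.
; It messages its linked Object, calls OnTrigger on the zombie AI controllers of actors tagged "Direct", then sends the trigger message to all delayed ceiling lights.
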(event `/Game/Selection/SelectionInterface.OnSelectionPress`
  (params (`Primitive Comp` :type "PrimitiveComponent Object Reference"))
  (`GameplayStatics.PlaySound2D` "/Game/Audio/Item/itempick2.itempick2" 0.25)
  (`/Engine/EditorBlueprintResources/StandardMacros.DoOnce` false
    (:`Completed`
      (message `/Game/Blueprints/ITrigger.On Trigger` (`self.Object`))
      (`|ExecutionSequence`
        (:`then_0`
          (bind _outactors (`GameplayStatics.GetAllActorsWithTag` "Direct"))
          (for _array_element _outactors
            (bind _returnvalue (`AIBlueprintHelperLibrary.GetAIController` _array_element))
            (bind _asbt_zombie_aicontroller_direct (cast `/Game/Blueprints/Zombie/BT_ZombieAIController_Direct` _returnvalue))
            (`/Game/Blueprints/Zombie/BT_ZombieAIController_Direct.On Trigger` _asbt_zombie_aicontroller_direct)))
        (:`then_1`
          (bind _outactors_2 (`GameplayStatics.GetAllActorsOfClass` "/Game/StarterContent/Blueprints/Blueprint_CeilingLight_Delay.Blueprint_CeilingLight_Delay_C"))
          (message `/Game/Blueprints/ITrigger.On Trigger` _outactors_2))))))

(fn `UserConstructionScript`)